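; Minimap capture actor that follows the first player from above and turns with the camera's heading.
; Each Tick it derives a yaw-only rotation from the player camera's forward vector, discarding pitch and roll.
; It then moves to the pawn's location, raised by a height variable and shifted along that heading by a center offset, so the captured area can sit off-center from the player.
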(event EventBeginPlay)

(event EventTick
  (params (DeltaSeconds :type Float%20%28single-precision%29))
  (bind _returnvalue (Game|GetPlayerCameraManager 0))
  (bind _returnvalue_2 (Game|Player|GetPlayerPawn 0))
  (bind _returnvalue_3 (Camera|GetCameraRotation _returnvalue))
  (bind _returnvalue_4 (Transformation|GetActorLocation _returnvalue_2))
  (bind _returnvalue_5 (Math|Rotator|GetRotationXVector _returnvalue_3))
  (bind (_x _y _z) (Math|Vector|BreakVector _returnvalue_4))
  (bind _yaw (Math|Vector|GetYawPitchfromVector _returnvalue_5))
  (bind _returnvalue_6 (Math|Rotator|MakeRotator 0.0 0.0 _yaw))
  (Transformation|SetActorRotation _returnvalue_6)
  (Transformation|SetActorLocation (+ (Math|Vector|RotateVector (Math|Vector|MakeVector (Variables|Default|GetMinimap%20Center%20Offset) 0.0 0.0) _returnvalue_6) (Math|Vector|MakeVector _x _y (+ _z (Variables|Default|GetMinimap%20Camera%20Height)))) false false))

(fn ConstructionScript)